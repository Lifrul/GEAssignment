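; BP_SendMessage shows one-time hint messages to the player on entering trigger areas on the second and third floors.
; BeginPlay sets the two hint strings about turning on lights and a powered game.
; Each trigger filters for the first-person character, fires once via DoOnce, and pushes its text into the controller's PlayerMessage widget.
; The widget is added to the viewport, then removed after a short delay.
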(event `self.Floor2.OnComponentBeginOverlap`
  (params (OverlappedComponent :type "PrimitiveComponent Object Reference") (OtherActor :type "Actor Object Reference") (OtherComp :type "PrimitiveComponent Object Reference") (OtherBodyIndex :type Integer) (bFromSweep :type Boolean) (SweepResult :type "HitResult Structure (by ref)"))
  (cast `/Game/FirstPerson/Blueprints/BP_FirstPersonCharacter` OtherActor)
  (`/Engine/EditorBlueprintResources/StandardMacros.DoOnce` false
    (:`Completed`
      (bind _asfirst_person_controller (cast `/Game/FirstPerson/Blueprints/FirstPersonController` (`GameplayStatics.GetPlayerController` 0)))
      (bind _playermessage (`/Game/FirstPerson/Blueprints/FirstPersonController.PlayerMessage` _asfirst_person_controller))
      (set `/Game/InterfaceWidgets/PlayerMessage.PlayerMessage` (`self.Floor2Message`) _playermessage)
      (`UserWidget.AddToViewport` _playermessage 0)
      (`KismetSystemLibrary.Delay` 5.0)
      (`Widget.RemoveFromParent` _playermessage))))

(event `self.Floor3.OnComponentBeginOverlap`
  (params (OverlappedComponent :type "PrimitiveComponent Object Reference") (OtherActor :type "Actor Object Reference") (OtherComp :type "PrimitiveComponent Object Reference") (OtherBodyIndex :type Integer) (bFromSweep :type Boolean) (SweepResult :type "HitResult Structure (by ref)"))
  (cast `/Game/FirstPerson/Blueprints/BP_FirstPersonCharacter` OtherActor)
  (`/Engine/EditorBlueprintResources/StandardMacros.DoOnce` false
    (:`Completed`
      (bind _asfirst_person_controller (cast `/Game/FirstPerson/Blueprints/FirstPersonController` (`GameplayStatics.GetPlayerController` 0)))
      (bind _playermessage (`/Game/FirstPerson/Blueprints/FirstPersonController.PlayerMessage` _asfirst_person_controller))
      (set `/Game/InterfaceWidgets/PlayerMessage.PlayerMessage` (`self.Floor3Message`) _playermessage)
      (`UserWidget.AddToViewport` _playermessage 0)
      (`KismetSystemLibrary.Delay` 5.0)
      (`Widget.RemoveFromParent` _playermessage))))

(event `self.ReceiveBeginPlay`
  (set `self.Floor2Message` "I think I need to turn on all the lights")
  (set `self.Floor3Message` "I think that game is hooked up to the power"))

(fn `UserConstructionScript`)