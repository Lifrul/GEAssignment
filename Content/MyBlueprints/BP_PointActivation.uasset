(event `self.ReceiveBeginPlay`)

(event `self.Sphere.OnComponentBeginOverlap`
  (params (OverlappedComponent :type "PrimitiveComponent Object Reference") (OtherActor :type "Actor Object Reference") (OtherComp :type "PrimitiveComponent Object Reference") (OtherBodyIndex :type Integer) (bFromSweep :type Boolean) (SweepResult :type "HitResult Structure (by ref)"))
  (cast `/Game/MyBlueprints/Bp_SkeeBall` OtherActor)
  (bind _asfirst_person_controller (cast `/Game/FirstPerson/Blueprints/FirstPersonController` (`GameplayStatics.GetPlayerController` 0)))
  (bind _ballpointswidget (`/Game/FirstPerson/Blueprints/FirstPersonController.BallPointsWidget` _asfirst_person_controller))
  (set `/Game/InterfaceWidgets/BallGamePointsWidget.Number` "10" _ballpointswidget)
  (`UserWidget.AddToViewport` _ballpointswidget 0))

(event `self.ReceiveTick`
  (params (DeltaSeconds :type "Float (single-precision)"))
  (bind _asfirst_person_controller (cast `/Game/FirstPerson/Blueprints/FirstPersonController` (`GameplayStatics.GetPlayerController` 0)))
  (set `/Game/InterfaceWidgets/BallGamePointsWidget.Number` (`KismetTextLibrary.Conv_DoubleToText` (`self.Points`) "HalfToEven") (`/Game/FirstPerson/Blueprints/FirstPersonController.BallPointsWidget` _asfirst_person_controller))
  (if (>= (`self.Points`) 350.0)
    (`GameplayStatics.DoesSaveGameExist` "")
    (if true
      (`GameplayStatics.DeleteGameInSlot` "save1")
      (`GameplayStatics.OpenLevel` "WinScene"))))

(fn `UserConstructionScript`)