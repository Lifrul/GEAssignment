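; BP_Spark is an actor that repeatedly spawns a P_Fire effect at its root until the saved game records that Floor2 was reached.
; From BeginPlay it loops on a random whole-second delay of up to five seconds, reloading the save slot before and after each wait to check Floor2Reached.
; If no save exists, it creates and writes a BP_SaveGame before entering the loop.
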(event `self.ReceiveBeginPlay`
  (bind _returnvalue (`GameplayStatics.DoesSaveGameExist` "save1" :!label _label))
  (if _returnvalue
    (bind _returnvalue_2 (`GameplayStatics.LoadGameFromSlot` "save1"))
    (bind _asbp_save_game (cast `/Game/MyBlueprints/BP_SaveGame` _returnvalue_2))
    (if (not (`/Game/MyBlueprints/BP_SaveGame.Floor2Reached` _asbp_save_game))
      (`KismetSystemLibrary.Delay` (`KismetMathLibrary.Conv_IntToDouble` (`KismetMathLibrary.RandomIntegerInRange` 0 5)) :!label _label_2)
      (bind _returnvalue_3 (`GameplayStatics.DoesSaveGameExist` "save1"))
      (if _returnvalue_3
        (bind _returnvalue_4 (`GameplayStatics.LoadGameFromSlot` "save1"))
        (bind _asbp_save_game_2 (cast `/Game/MyBlueprints/BP_SaveGame` _returnvalue_4))
        (if (not (`/Game/MyBlueprints/BP_SaveGame.Floor2Reached` _asbp_save_game_2))
          (`GameplayStatics.SpawnEmitterAtLocation` "/Game/StarterContent/Particles/P_Fire.P_Fire" (`SceneComponent.K2_GetComponentLocation` (`self.DefaultSceneRoot`)) (struct) (1.0 1.0 1.0) true "AutoRelease")
          (goto _label))))
    (else
      (bind _returnvalue_5 (`GameplayStatics.CreateSaveGameObject` "/Game/MyBlueprints/BP_SaveGame.BP_SaveGame_C"))
      (`GameplayStatics.SaveGameToSlot` _returnvalue_5 "save1")
      (bind _asbp_save_game_3 (cast `/Game/MyBlueprints/BP_SaveGame` _returnvalue_5))
      (set `/Game/MyBlueprints/BP_SaveGame.Floor2Reached` false _asbp_save_game_3)
      (goto _label_2))))

(fn `UserConstructionScript`)