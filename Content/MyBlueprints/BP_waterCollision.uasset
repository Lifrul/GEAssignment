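; BP_waterCollision is a box trigger that kills the player with a fire effect and ends the game.
; On any overlap it loads the "save1" slot and acts only if Floor2Reached is false in BP_SaveGame.
; It then plays a fire sound and particle at the player's location and, after a short delay, opens the GameOver level.
; The overlapping actor is not checked, and the character cast on BeginPlay leads to nothing.
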(event `self.ReceiveBeginPlay`
  (cast `/Game/FirstPerson/Blueprints/BP_FirstPersonCharacter` (`GameplayStatics.GetPlayerCharacter` 0)))

(event `self.Box.OnComponentBeginOverlap`
  (params (OverlappedComponent :type "PrimitiveComponent Object Reference") (OtherActor :type "Actor Object Reference") (OtherComp :type "PrimitiveComponent Object Reference") (OtherBodyIndex :type Integer) (bFromSweep :type Boolean) (SweepResult :type "HitResult Structure (by ref)"))
  (bind _returnvalue (`self.K2_GetActorLocation` (`GameplayStatics.GetPlayerCharacter` 0)))
  (bind _returnvalue_2 (`GameplayStatics.LoadGameFromSlot` "save1"))
  (bind _asbp_save_game (cast `/Game/MyBlueprints/BP_SaveGame` _returnvalue_2))
  (if (not (`/Game/MyBlueprints/BP_SaveGame.Floor2Reached` _asbp_save_game))
    (`GameplayStatics.PlaySoundAtLocation` "/Game/StarterContent/Audio/Fire01_Cue.Fire01_Cue" _returnvalue (struct) 1.0 1.0 0.0 null null null null)
    (`GameplayStatics.SpawnEmitterAtLocation` "/Game/StarterContent/Particles/P_Fire.P_Fire" _returnvalue)
    (`KismetSystemLibrary.Delay` 0.8)
    (`GameplayStatics.OpenLevel` "GameOver")))

(fn `UserConstructionScript`)