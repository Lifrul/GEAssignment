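; BP_PowerBox is a power box that activates the elevator when the first-person character enters its trigger holding a tool.
; With a tool, it sets Floor2Reached in the existing "save1" save, writes it back and reports the elevator active.
; Without an existing save, it only creates a save object in memory, without writing it or showing a message.
; Without a tool, a timed on-screen message says a wrench is needed.
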(event `self.ReceiveBeginPlay`
  (bind _asbp_first_person_character (cast `/Game/FirstPerson/Blueprints/BP_FirstPersonCharacter` (`GameplayStatics.GetPlayerCharacter` 0)))
  (set `self.ThePlayer` _asbp_first_person_character))

(event `self.Box.OnComponentBeginOverlap`
  (params (OverlappedComponent :type "PrimitiveComponent Object Reference") (OtherActor :type "Actor Object Reference") (OtherComp :type "PrimitiveComponent Object Reference") (OtherBodyIndex :type Integer) (bFromSweep :type Boolean) (SweepResult :type "HitResult Structure (by ref)"))
  (bind _asbp_first_person_character (cast `/Game/FirstPerson/Blueprints/BP_FirstPersonCharacter` OtherActor))
  (if (`/Game/FirstPerson/Blueprints/BP_FirstPersonCharacter.HoldingTool` _asbp_first_person_character)
    (bind _returnvalue (`GameplayStatics.DoesSaveGameExist` "save1"))
    (if _returnvalue
      (bind _returnvalue_2 (`GameplayStatics.LoadGameFromSlot` "save1"))
      (bind _asbp_save_game (cast `/Game/MyBlueprints/BP_SaveGame` _returnvalue_2))
      (bind _output_get (set `self.Save` _asbp_save_game))
      (set `/Game/MyBlueprints/BP_SaveGame.Floor2Reached` true _output_get)
      (`GameplayStatics.SaveGameToSlot` _output_get "save1")
      (`KismetSystemLibrary.PrintString` "game saved")
      (bind _asfirst_person_controller (cast `/Game/FirstPerson/Blueprints/FirstPersonController` (`GameplayStatics.GetPlayerController` 0)))
      (bind _playermessage (`/Game/FirstPerson/Blueprints/FirstPersonController.PlayerMessage` _asfirst_person_controller))
      (set `/Game/InterfaceWidgets/PlayerMessage.PlayerMessage` "Elevator is active" _playermessage)
      (`UserWidget.AddToViewport` _playermessage 0)
      (`KismetSystemLibrary.Delay` 5.0)
      (`Widget.RemoveFromParent` _playermessage)
      (else
        (bind _returnvalue_3 (`GameplayStatics.CreateSaveGameObject` "/Game/MyBlueprints/BP_SaveGame.BP_SaveGame_C"))
        (set `/Game/MyBlueprints/BP_SaveGame.Floor2Reached` true _returnvalue_3)
        (set `/Game/MyBlueprints/BP_SaveGame.Floor3Reached` false _returnvalue_3)
        (set `self.Save` _returnvalue_3)))
    (else
      (bind _asfirst_person_controller_2 (cast `/Game/FirstPerson/Blueprints/FirstPersonController` (`GameplayStatics.GetPlayerController` 0)))
      (bind _playermessage_2 (`/Game/FirstPerson/Blueprints/FirstPersonController.PlayerMessage` _asfirst_person_controller_2))
      (set `/Game/InterfaceWidgets/PlayerMessage.PlayerMessage` "You need a wrench" _playermessage_2)
      (`UserWidget.AddToViewport` _playermessage_2 0)
      (`KismetSystemLibrary.Delay` 5.0)
      (`Widget.RemoveFromParent` _playermessage_2))))

(fn `UserConstructionScript`)