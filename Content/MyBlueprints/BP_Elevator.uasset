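; BP_Elevator is an elevator that carries the first-person character between floors, gated by floor progress in the "save1" save game.
; On BeginPlay it reads the save and plays timelines to move the mesh up to the saved floor, setting 2ND and Final flags.
; On player overlap it reloads the save and, unless the matching flag is set, plays that floor's timeline with delayed-stop audio.
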(event `self.ElevatorContact.OnComponentBeginOverlap`
  (params (OverlappedComponent :type "PrimitiveComponent Object Reference") (OtherActor :type "Actor Object Reference") (OtherComp :type "PrimitiveComponent Object Reference") (OtherBodyIndex :type Integer) (bFromSweep :type Boolean) (SweepResult :type "HitResult Structure (by ref)"))
  (bind _audio (`self.Audio`))
  (bind _returnvalue (`GameplayStatics.LoadGameFromSlot` "save1"))
  (bind _asbp_save_game (cast `/Game/MyBlueprints/BP_SaveGame` _returnvalue))
  (cast `/Game/FirstPerson/Blueprints/BP_FirstPersonCharacter` OtherActor)
  (if (`/Game/MyBlueprints/BP_SaveGame.Floor2Reached` _asbp_save_game)
    (if (`/Game/MyBlueprints/BP_SaveGame.Floor3Reached` _asbp_save_game)
      (if (not (`self.Final`))
        (`AudioComponent.Play` _audio 0.0)
        (`KismetSystemLibrary.Delay` 0.2)
        (`/Engine/EditorBlueprintResources/StandardMacros.DoOnce` false
          (:`Completed`
            (bind (_direction _elevevtor_floor1) (`Timeline|Timeline_1`)
              (:`Update`
                (`SceneComponent.K2_SetRelativeLocation` (`self.ElevatorMesh`) _elevevtor_floor1 false false)
                (set `self.Final` true)
                (`AudioComponent.StopDelayed` _audio 1.5))))))
      (elif (not (`self.2ND`))
        (`AudioComponent.Play` _audio 0.0)
        (`KismetSystemLibrary.Delay` 0.2)
        (`/Engine/EditorBlueprintResources/StandardMacros.DoOnce` false
          (:`Completed`
            (bind (_direction_2 _elevevtor_floor1_2) (`Timeline|Elevator`)
              (:`Update`
                (`SceneComponent.K2_SetRelativeLocation` (`self.ElevatorMesh`) _elevevtor_floor1_2 false false)
                (`AudioComponent.StopDelayed` _audio 1.5)))))))))

(event `self.ReceiveBeginPlay`
  (set `self.2ND` false)
  (bind _returnvalue (`GameplayStatics.DoesSaveGameExist` "save1"))
  (if _returnvalue
    (bind _returnvalue_2 (`GameplayStatics.LoadGameFromSlot` "save1"))
    (bind _asbp_save_game (cast `/Game/MyBlueprints/BP_SaveGame` _returnvalue_2))
    (if (`/Game/MyBlueprints/BP_SaveGame.Floor2Reached` _asbp_save_game)
      (`KismetSystemLibrary.Delay` 0.2)
      (`/Engine/EditorBlueprintResources/StandardMacros.DoOnce` false
        (:`Completed`
          (bind (_direction _elevevtor_floor1) (`Timeline|Timeline_0`)
            (:`Update`
              (`SceneComponent.K2_SetRelativeLocation` (`self.ElevatorMesh`) _elevevtor_floor1 false false)
              (set `self.2ND` true)
              (if (`/Game/MyBlueprints/BP_SaveGame.Floor3Reached` _asbp_save_game)
                (bind (_direction_2 _elevevtor_floor1_2) (`Timeline|Timeline`)
                  (:`Update`
                    (`SceneComponent.K2_SetRelativeLocation` (`self.ElevatorMesh`) _elevevtor_floor1_2 false false)
                    (set `self.Final` true)))))))))))

(fn `UserConstructionScript`)